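; Player controller for the village that sets up mouse-driven game-and-UI input and routes player input to the village HUD.
; On BeginPlay it caches the village character and HUD, adds the village Enhanced Input mapping context, and binds to CommonInput device changes, storing and debug-printing the current input type.
; Holding Back past a time threshold leaves the building, with hold time tracked, and a debug key toggles the inventory.
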(event Custom|OnInputDeviceChanged
  (params (bNewInputType :type ECommonInputType%20Enum :default "MouseAndKeyboard"))
  ;[1 1 1] bind on input device changed
  (CallFunction|NewInputType bNewInputType))

(event Custom|NewInputType
  (params (Input%20Type :type ECommonInputType%20Enum :default "MouseAndKeyboard"))
  (bind _output_get (Variables|Default|SetCurrent%20Input%20Type Input%20Type))
  (CallFunction|PrintDebugMessage "None" "" (Utilities|String|EnumtoString _output_get) "" 2e+01 "NewEnumerator12"))

(event Input|EnhancedActionEvents|EnhancedInputActionIA_Back
  (params (ActionValue :type Boolean) (ElapsedSeconds :type Float%20%28double-precision%29) (TriggeredSeconds :type Float%20%28double-precision%29) (InputAction :type Input%20Action%20Object%20Reference :default "/Game/Programming/InputMappings/HuntForest/IA_Back.IA_Back"))
  ;[1 1 1] back
  (:Triggered
    (Variables|Default|SetSeconds_BackTriggered TriggeredSeconds)
    (if (>= TriggeredSeconds (Variables|Default|GetPress%20for%20Seconds))
      (Default|LeaveBuilding (Variables|Default|GetBP_HUD))))
  (:Completed
    (Variables|Default|SetSeconds_BackTriggered 0.0)))

(event EventBeginPlay
  (bind _returnvalue (PlayerController|LocalPlayerSubsystems|GetEnhancedInputLocalPlayerSubsystem))
  (Input|SetInputModeGameandUI self 0 "DoNotLock" true false)
  (Variables|Default|SetbShowMouseCursor true)
  (Variables|Default|SetbEnableMouseOverEvents true)
  (Variables|Default|SetbEnableClickEvents true)
  (bind _asbp_main_characte_village (Utilities|Casting|CastToBP_MainCharacte_Village (Game|GetPlayerCharacter 0)))
  (Variables|Default|SetBP_Player _asbp_main_characte_village)
  (bind _asbp_hud_village (Utilities|Casting|CastToBP_HUD_Village (HUD|GetHUD))
    (:then
      (Variables|Default|SetBP_HUD _asbp_hud_village)
      ;[1 1 1] mapping contect
      (Utilities|IsValid _returnvalue
        (:Is%20Valid
          (Input|AddMappingContext _returnvalue "/Game/Programming/InputMappings/Village/InputMap_Village.InputMap_Village" 0 "(bIgnoreAllPressedKeysUntilRelease=True,bForceImmediately=False)")
          ;[1 1 1] bind on input device changed
          (EventDispatchers|BindEventtoOnInputMethodChanged (PlayerController|LocalPlayerSubsystems|GetCommonInputSubsystem) (delegate Custom|OnInputDeviceChanged)))))
    (:CastFailed
      (CallFunction|PrintDebugMessage "None" "Cast To HUD failed" "" "" 0.0 "NewEnumerator13"))))

(event Input|KeyboardEvents|DebugKeyI
  (params (Key :type Key%20Structure :default "None") (ActionValue :type Input%20Action%20Value%20Structure))
  (:Pressed
    (Default|ToggleInventory (Variables|Default|GetBP_HUD))))

(fn ConstructionScript)