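; Base pickup actor for items in the spatial inventory system.
; On BeginPlay it fills a missing ItemObject from GetDefaultItemObject, which is empty in this base class.
; When BP_MainCharacter overlaps its sphere, it passes ItemObject to that character's SpacialInventoryComponent via TryAddItem, prints the result and destroys itself on success.
; The character is found by a direct cast, with a todo to switch to an interface.
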(event `self.ReceiveBeginPlay`
  (`self.ItemObject`
    (:`then`)
    (:`else`
      (bind _itemobject (`self.GetDefaultItemObject`))
      (set `self.ItemObject` _itemobject))))

(event `self.Sphere.OnComponentBeginOverlap`
  (params (OverlappedComponent :type "PrimitiveComponent Object Reference") (OtherActor :type "Actor Object Reference") (OtherComp :type "PrimitiveComponent Object Reference") (OtherBodyIndex :type Integer) (bFromSweep :type Boolean) (SweepResult :type "HitResult Structure (by ref)"))
  ;[1 0 0] todo: make this an interface
  (bind _asbp_main_character (cast `/Game/Programming/Blueprints/BP_MainCharacter` OtherActor))
  (bind _added (`/Game/Programming/Blueprints/Inventory/Spacial-System/SpacialInventoryComponent.Try Add Item` (`/Game/Programming/Blueprints/BP_MainCharacter.SpacialInventoryComponent` _asbp_main_character) (`self.ItemObject`)))
  (`/Game/Programming/Libraries_Enums_Interfaces/FL_Debug.PrintDebugMessage` "None" "Added Item: " (`KismetStringLibrary.Conv_BoolToString` _added) "" 10.0 "NewEnumerator15")
  (if _added
    (`self.K2_DestroyActor`)))

(fn `GetDefaultItemObject`
  (returns (ItemObject :type "/Game/Programming/Blueprints/Inventory/Spacial-System/BP_ItemObjectBase Object Reference"))
  (return null))

(fn `UserConstructionScript`)