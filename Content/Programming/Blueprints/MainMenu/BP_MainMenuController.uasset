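; Player controller for the main menu that sets up menu input and creates the main menu widget.
; On BeginPlay it adds the menu mapping context, shows WB_MainMenu with the cursor visible, and sets Game and UI input focused on the widget.
; Enhanced Input actions for back, apply and switching settings cards up or down are forwarded directly to the widget.
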(event `self.ReceiveBeginPlay`
  (bind _returnvalue (subsystem `EnhancedInputLocalPlayerSubsystem`))
  ;[1 1 1] mapping contect
  (`/Engine/EditorBlueprintResources/StandardMacros.IsValid` _returnvalue
    (:`Is Valid`
      (`EnhancedInputSubsystemInterface.AddMappingContext` _returnvalue "/Game/Programming/InputMappings/MainMenu/InputMap_Menu.InputMap_Menu" 0 (struct))
      (bind _returnvalue_2 (`|CreateWidget` "/Game/Programming/Blueprints/Widgets/WB_MainMenu.WB_MainMenu_C" self))
      (bind _output_get (set `self.Widget_MainMenu` _returnvalue_2))
      (`UserWidget.AddToViewport` _output_get 0)
      (`WidgetBlueprintLibrary.SetInputMode_GameAndUIEx` self _output_get)
      (set `self.bShowMouseCursor` true))))

(event `EnhancedInput|/Game/Programming/InputMappings/HuntForest/IA_Back`
  (params (ActionValue :type Boolean) (ElapsedSeconds :type "Float (double-precision)") (TriggeredSeconds :type "Float (double-precision)") (InputAction :type "InputAction Object Reference" :default "/Game/Programming/InputMappings/HuntForest/IA_Back.IA_Back"))
  (:`Started`
    (`/Game/Programming/Blueprints/Widgets/WB_MainMenu.Back` (`self.Widget_MainMenu`))))

(event `EnhancedInput|/Game/Programming/InputMappings/MainMenu/IA_Apply`
  (params (ActionValue :type Boolean) (ElapsedSeconds :type "Float (double-precision)") (TriggeredSeconds :type "Float (double-precision)") (InputAction :type "InputAction Object Reference" :default "/Game/Programming/InputMappings/MainMenu/IA_Apply.IA_Apply"))
  (:`Started`
    (`/Game/Programming/Blueprints/Widgets/WB_MainMenu.Apply` (`self.Widget_MainMenu`))))

(event `EnhancedInput|/Game/Programming/InputMappings/MainMenu/IA_ChangeCardUp`
  (params (ActionValue :type Boolean) (ElapsedSeconds :type "Float (double-precision)") (TriggeredSeconds :type "Float (double-precision)") (InputAction :type "InputAction Object Reference" :default "/Game/Programming/InputMappings/MainMenu/IA_ChangeCardUp.IA_ChangeCardUp"))
  (:`Started`
    (`/Game/Programming/Blueprints/Widgets/WB_MainMenu.ChangeSettingsCard` (`self.Widget_MainMenu`) true)))

(event `EnhancedInput|/Game/Programming/InputMappings/MainMenu/IA_ChangeCardDown`
  (params (ActionValue :type Boolean) (ElapsedSeconds :type "Float (double-precision)") (TriggeredSeconds :type "Float (double-precision)") (InputAction :type "InputAction Object Reference" :default "/Game/Programming/InputMappings/MainMenu/IA_ChangeCardDown.IA_ChangeCardDown"))
  (:`Started`
    (`/Game/Programming/Blueprints/Widgets/WB_MainMenu.ChangeSettingsCard` (`self.Widget_MainMenu`) false)))

(fn `UserConstructionScript`)