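; BP_Wind is a wind actor that keeps a wind sound's modulation in step with the WindParameter material parameter collection.
; On BeginPlay it sets a high WindIntensity, activates its Audio component and passes the value read back to the sound's "Mod Level" parameter.
; After a fixed delay it lowers the intensity and pushes it again, a one-time scripted change with no per-tick updates.
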(event `self.ReceiveBeginPlay`
  (`KismetMaterialLibrary.SetScalarParameterValue` "/Game/Art/Props/Materials/Parameters/WindParameter.WindParameter" "WindIntensity" 5.0)
  (`ActorComponent.Activate` (`self.Audio`) false)
  (bind _returnvalue (`KismetMaterialLibrary.GetScalarParameterValue` "/Game/Art/Props/Materials/Parameters/WindParameter.WindParameter" "WindIntensity"))
  (`AudioComponent.SetFloatParameter` (`self.Audio`) "Mod Level" _returnvalue)
  (`KismetSystemLibrary.Delay` 10.0)
  (`KismetMaterialLibrary.SetScalarParameterValue` "/Game/Art/Props/Materials/Parameters/WindParameter.WindParameter" "WindIntensity" 0.5)
  (bind _returnvalue_2 (`KismetMaterialLibrary.GetScalarParameterValue` "/Game/Art/Props/Materials/Parameters/WindParameter.WindParameter" "WindIntensity"))
  (`AudioComponent.SetFloatParameter` (`self.Audio`) "Mod Level" _returnvalue_2))

(fn `UserConstructionScript`)