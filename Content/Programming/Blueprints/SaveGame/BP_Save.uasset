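; Save object that stores and restores the player's quest log and per-quest progress.
; SaveQuestLog copies the active and completed quest lists, while SaveQuestDetails records each quest's current stage and objective progress in a map keyed by quest ID.
; LoadQuests re-adds each active quest through the quest log component, applies its saved stage and progress, then overwrites the component's active and completed lists with the saved ones.
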(fn `LoadQuests`
  (params (Questlog :type "/Game/Programming/Blueprints/Questsystem/Questlog_Component Object Reference"))
  (for _array_element (`self.CurrentActiveQuests`)
    (bind _returnvalue (`/Game/Programming/Blueprints/Questsystem/Questlog_Component.Add New Quest` Questlog _array_element))
    (bind (_progress _currentstage) (break `/Game/Programming/Blueprints/SaveGame/F_QuestSaveData` (`BlueprintMapLibrary.Map_Find` (`self.QuestProgress`) _array_element)))
    (set `/Game/Programming/Blueprints/Questsystem/BP_Quest_Base.CurrentStage` _currentstage _returnvalue)
    (set `/Game/Programming/Blueprints/Questsystem/BP_Quest_Base.CurrentObjectiveProgress` _progress _returnvalue))
  (set `/Game/Programming/Blueprints/Questsystem/Questlog_Component.CurrentActiveQuest` (`self.CurrentActiveQuests`) Questlog)
  (set `/Game/Programming/Blueprints/Questsystem/Questlog_Component.CompletedQuest` (`self.CompletedQuests`) Questlog))

(fn `Save Quest Log`
  (params (`Questlog Component` :type "/Game/Programming/Blueprints/Questsystem/Questlog_Component Object Reference"))
  (set `self.CurrentActiveQuests` (`/Game/Programming/Blueprints/Questsystem/Questlog_Component.CurrentActiveQuest` `Questlog Component`))
  (set `self.CompletedQuests` (`/Game/Programming/Blueprints/Questsystem/Questlog_Component.CompletedQuest` `Questlog Component`)))

(fn `SaveQuestDetails`
  (params (Quest :type "/Game/Programming/Blueprints/Questsystem/BP_Quest_Base Object Reference"))
  (`BlueprintMapLibrary.Map_Add` (`self.QuestProgress`) (`/Game/Programming/Blueprints/Questsystem/BP_Quest_Base.QuestID` Quest) (make `/Game/Programming/Blueprints/SaveGame/F_QuestSaveData` (`/Game/Programming/Blueprints/Questsystem/BP_Quest_Base.CurrentObjectiveProgress` Quest) (`/Game/Programming/Blueprints/Questsystem/BP_Quest_Base.CurrentStage` Quest))))