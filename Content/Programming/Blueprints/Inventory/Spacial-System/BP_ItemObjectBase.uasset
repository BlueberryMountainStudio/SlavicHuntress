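; BP_ItemObjectBase is the base item object for a spatial inventory system, holding an item's icons, size, rotation state and descriptive data.
; Rotate toggles the Rotated flag, which makes GetItemIcon return the rotated icon and GetDimensions swap X and Y.
; GetAllItemInfos returns the item's name, value, resource and description in one call.
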(fn `Get All ItemInfos`
  (returns (Name :type Text) (Value :type Integer) (Ressource :type Text) (Description :type Text))
  (return (`self.Name`) (`self.Value`) (`self.Ressource`) (`self.Description`)))

(fn `Get Dimensions`
  (returns (Dimensions :type "IntPoint Structure"))
  (bind (_dimensions_x _dimensions_y) (break `IntPoint` (`self.Dimensions`)))
  (bind (_dimensions_x_2 _dimensions_y_2) (break `IntPoint` (`self.Dimensions`)))
  (if (`self.Rotated`)
    (return (make `IntPoint` _dimensions_y _dimensions_x))
    (else
      (return (make `IntPoint` _dimensions_x_2 _dimensions_y_2)))))

(fn `Get Item Icon`
  (returns (Icon :type "MaterialInterface Object Reference"))
  (return (select `bool` (`self.Rotated`) :`false` (`self.Icon`) :`true` (`self.IconRotated`))))

(fn `Rotate`
  (set `self.Rotated` (not (`self.Rotated`)))
  (return))