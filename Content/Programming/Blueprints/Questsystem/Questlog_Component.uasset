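; Quest log component that keeps the list of active quests.
; Adding a quest stores its ID uniquely, spawns a BP_Quest_Base actor for it, appends that actor to the current quests array and prints a debug message.
; The spawn runs even when the ID is already listed.
; A query reports whether an ID is active, while completing and tracking quests are empty stubs.
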(fn `Add New Quest`
  (params (`Quest ID` :type Name))
  ;[1 1 1] add unique so we dont get dduplicates
  (`KismetArrayLibrary.Array_AddUnique` (`self.CurrentActiveQuest`) `Quest ID`)
  ;[1 1 1] add a questactor for it to the questactor array
  (bind _returnvalue (`|SpawnActorFromClass` "/Game/Programming/Blueprints/Questsystem/BP_Quest_Base.BP_Quest_Base_C" (`KismetMathLibrary.MakeTransform` (0.0 0.0 0.0)) "Undefined" "MultiplyWithRoot" null `Quest ID` null))
  (`KismetArrayLibrary.Array_Add` (`self.CurrentQuests`) _returnvalue)
  (`/Game/Programming/Libraries_Enums_Interfaces/FL_Debug.PrintDebugMessage` "None" "Added Quest: " (`KismetStringLibrary.Conv_NameToString` (`local.Quest ID`)) "" 20.0 "NewEnumerator20"))

(fn `Complete Quest`)

(fn `Query Active Quest`
  (params (`Quest ID` :type Name))
  (returns (ReturnValue :type Boolean))
  (return (`KismetArrayLibrary.Array_Contains` (`self.CurrentActiveQuest`) `Quest ID`)))

(fn `Track Quest`)