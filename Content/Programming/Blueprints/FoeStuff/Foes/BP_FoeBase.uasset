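; Base foe actor that tracks health and a three-slot alert status, ending in death or fleeing.
; BeginPlay scatters footprint tracks in a ring around the foe and creates the loot widget.
; Damage reaching zero health or a full last alert slot shows that widget with the matching outcome.
; Cursor hover works while highlighted; a spacing-aware track spawner exists but is not called here.
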(event `self.ReceiveBeginPlay`
  (`self.SpawnAllTracks`)
  ;[1 1 1] set reference to loot widget
  (bind _returnvalue (`|CreateWidget` "/Game/Programming/Blueprints/Widgets/WB_LootMessage.WB_LootMessage_C" (`GameplayStatics.GetPlayerController` 0)))
  (bind _output_get (set `self.WB_Loot` _returnvalue))
  (`UserWidget.AddToViewport` _output_get 3))

(event `self.ReceiveTick`
  (params (DeltaSeconds :type "Float (single-precision)"))
  (`/Game/Programming/Libraries_Enums_Interfaces/FL_Debug.PrintDebugMessage` "None" (`KismetSystemLibrary.GetDisplayName` self) ": " (`KismetStringLibrary.Conv_DoubleToString` (`self.currentHealth`)) 0.0 "NewEnumerator17"))

(event `self.mesh.OnBeginCursorOver`
  (params (TouchedComponent :type "PrimitiveComponent Object Reference"))
  (if (`self.highlighted`)
    (`self.Hover` true)))

(event `self.mesh.OnEndCursorOver`
  (params (TouchedComponent :type "PrimitiveComponent Object Reference"))
  (`self.Hover` false))

(event `self.ReceiveAnyDamage`
  (params (Damage :type "Float (single-precision)") (DamageType :type "DamageType Object Reference") (InstigatedBy :type "Controller Object Reference") (DamageCauser :type "Actor Object Reference"))
  (set `self.currentHealth` (- (`self.currentHealth`) Damage))
  (if (`self.Check Is 0 HP`)
    (`self.FoeDied`)))

(fn `Check Is 0 HP`
  (returns (ReturnValue :type Boolean))
  (return (<= (`self.currentHealth`) 0.0)))

(fn `CheckAlertStatus`
  (params (Array :type "Array of Float (double-precision)"))
  (returns (Fled :type Boolean))
  (if (>= (`|GetArrayItem` Array 2) 100.0)
    (return true)))

(fn `FillNextAlert`
  (returns (AlertStatus :type "Array of Float (double-precision)"))
  (bind _alertstatus (`self.AlertStatus`))
  (bind _alertstatus_2 (`self.AlertStatus`))
  (bind _alertstatus_3 (`self.AlertStatus`))
  ;[1 1 1] check index 0
  (if (== (`|GetArrayItem` _alertstatus) 100.0)
    ;[1 1 1] check index 1
    (if (== (`|GetArrayItem` _alertstatus_3 1) 100.0)
      ;[1 1 1] check index 2
      (if (== (`|GetArrayItem` _alertstatus_2 2) 100.0)
        (return (`self.AlertStatus`))
        (else
          (`KismetArrayLibrary.Array_Set` _alertstatus_2 2 100.0)
          (return (`self.AlertStatus`))))
      (else
        (`KismetArrayLibrary.Array_Set` _alertstatus_3 1 100.0)
        (return (`self.AlertStatus`))))
    (else
      (`KismetArrayLibrary.Array_Set` _alertstatus 0 100.0)
      (return (`self.AlertStatus`)))))

(fn `FoeDied`
  (set `self.IsDead` true)
  (`/Game/Programming/Blueprints/Widgets/WB_LootMessage.Update Content` (`self.WB_Loot`) 0 (`self.Loot`) true)
  (return))

(fn `FoeFled`
  (set `self.IsFled` true)
  (`/Game/Programming/Blueprints/Widgets/WB_LootMessage.Update Content` (`self.WB_Loot`) 1 (`self.Loot`) true)
  (return))

(fn `SpawnAllTracks`
  ;[1 1 1] as long as max amount of tracks isnt met spawn another track
  (if (< (`self.CurrentAmountOfTracks`) (`self.Max_AmountOfTracks`)) :!label _label
    (`self.SpawnSingleTrack`)
    (`/Engine/EditorBlueprintResources/StandardMacros.IncrementFloat` (`self.CurrentAmountOfTracks`)
      (:`  `
        (goto _label)))))

(fn `SpawnSingleTrack`
  (bind (_returnvalue_location _returnvalue_rotation _returnvalue_scale) (`KismetMathLibrary.BreakTransform` (`self.GetTransform`)))
  (bind (_output_itemid _output_quantity _output_image) (break `/Game/Programming/Blueprints/Inventory/F_SlotStruct` (`|GetArrayItem` (`self.Loot`))))
  ;[1 1 1] get random location
  (bind (_x _y) (`/Game/Programming/Libraries_Enums_Interfaces/FL_Misc.Get Random Point In Circle` _returnvalue_location (`self.Min_TrackSpawnRadius`) (`self.Max_TrackSpawnRadius`)))
  (`|SpawnActorFromClass` "/Game/Programming/Blueprints/FoeStuff/Tracks/BP_TrackFoodprint.BP_TrackFoodprint_C" (`KismetMathLibrary.MakeTransform` (`KismetMathLibrary.MakeVector` _x _y (+ (`.Z` (`KismetMathLibrary.BreakVector3f` _returnvalue_location)) 20.0)) _returnvalue_rotation _returnvalue_scale) "AdjustIfPossibleButAlwaysSpawn" "MultiplyWithRoot" null self (`self.Widget_HeaderImage`) _output_image null))

(fn `SpawnSingleTrackWithDistance`
  (returns (Spawned :type Boolean))
  (locals (DesiredLocation_Local :type "Vector Structure") (LoopCounter_Local :type Integer) (CanSpawn_Local :type Boolean))
  (bind (_returnvalue_location _returnvalue_rotation _returnvalue_scale) (`KismetMathLibrary.BreakTransform` (`self.GetTransform`)))
  (bind _min_spawndistance (`self.Min_SpawnDistance`))
  (bind _desiredlocation_local (`local.DesiredLocation_Local`))
  (`|ExecutionSequence`
    (:`then_0`
      ;[1 1 1] find all tracks that have already spawned
      (bind _outactors (`GameplayStatics.GetAllActorsWithTag` "Track"))
      (for _array_element _outactors
        (`KismetArrayLibrary.Array_AddUnique` (`self.SpawnedTracksLocation`) (`self.K2_GetActorLocation` _array_element))))
    (:`then_1`
      ;[1 1 1] only try 100 times to find a location
      (if (< (`local.LoopCounter_Local`) 100) :!label _label
        ;[1 1 1] get random location
        (bind (_x _y) (`/Game/Programming/Libraries_Enums_Interfaces/FL_Misc.Get Random Point In Circle` _returnvalue_location (`self.Min_TrackSpawnRadius`) (`self.Max_TrackSpawnRadius`)))
        (set `local.DesiredLocation_Local` (`KismetMathLibrary.MakeVector` _x _y (+ (`.Z` (`KismetMathLibrary.BreakVector3f` _returnvalue_location)) 20.0)))
        ;[1 1 1] check if desired location has min distance to other track locations
        (for (_array_element_2 _array_index) (`self.SpawnedTracksLocation`)
          (`/Game/Programming/Libraries_Enums_Interfaces/FL_Debug.PrintDebugMessage` "None" "" (`KismetStringLibrary.Conv_VectorToString` (- _desiredlocation_local _array_element_2)) "" 10.0 "NewEnumerator18")
          (bind (_x_2 _y_2) (`KismetMathLibrary.BreakVector3f` (- _desiredlocation_local _array_element_2)))
          (if (and (> _x_2 _min_spawndistance) (> _y_2 _min_spawndistance))
            (set `local.CanSpawn_Local` true)
            (`/Game/Programming/Libraries_Enums_Interfaces/FL_Debug.PrintDebugMessage` "None" "true" "" "" 10.0)
            (else
              (set `local.CanSpawn_Local` false)
              (`/Game/Programming/Libraries_Enums_Interfaces/FL_Debug.PrintDebugMessage` "None" "false" "" "" 10.0))))
        ;[1 1 1] check if actor can spawn, if not restart loop
        (if (`local.CanSpawn_Local`)
          (`|SpawnActorFromClass` "/Game/Programming/Blueprints/FoeStuff/Tracks/BP_TrackFoodprint.BP_TrackFoodprint_C" (`KismetMathLibrary.MakeTransform` (`local.DesiredLocation_Local`) _returnvalue_rotation _returnvalue_scale) "AdjustIfPossibleButAlwaysSpawn" "MultiplyWithRoot" null self (struct) (struct) null)
          (`KismetArrayLibrary.Array_Clear` (`self.SpawnedTracksLocation`))
          (return (`local.CanSpawn_Local`))
          (else
            (`/Engine/EditorBlueprintResources/StandardMacros.IncrementInt` (`local.LoopCounter_Local`)
              (:`  `
                (goto _label)))))))))

(fn `UpdateAlertStatus`
  (params (AlertStatus :type "Array of Float (double-precision)"))
  (returns (Fled :type Boolean))
  (bind _output_get (set `self.AlertStatus` AlertStatus))
  (bind _fled (`self.CheckAlertStatus` _output_get))
  (if _fled
    (`self.FoeFled`)
    (return true)
    (else
      (return false))))

(fn `UserConstructionScript`)