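; Base quest Blueprint that tracks objective progress for the current stage of one quest.
; On BeginPlay it loads the QuestID row from a data table, builds a progress map keyed by objective ID, and binds to the main character's objective event.
; Collection objectives are seeded from the player's inventory.
; OnObjectiveIDHeard adjusts counts up or down, re-evaluating IsCompleted against required quantities only on increases.
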(event `self.ReceiveBeginPlay`
  (`self.Get Quest Details`)
  (bind _asbp_main_character (cast `/Game/Programming/Blueprints/BP_MainCharacter` (`GameplayStatics.GetPlayerCharacter` 0)))
  (add `/Game/Programming/Blueprints/BP_MainCharacter.OnObjectiveIDCalled` _asbp_main_character (`|CreateDelegate` :!event `On Objective ID Heard`))
  ;[1 1 1] only go further with collection quests
  (for _array_element (`.Objectives_20_0560FE6442A69F718DC381889D24ED81` (break `/Game/Programming/Blueprints/Questsystem/F_StageDetails` (`self.CurrentStageDetails`)))
    (bind (_objectivename _description _type _objectiveid) (break `/Game/Programming/Blueprints/Questsystem/F_ObjectiveDetails` _array_element))
    (if (`|EnumEquality` _type "NewEnumerator3")
      (bind _asbp_main_character_2 (cast `/Game/Programming/Blueprints/BP_MainCharacter` (`GameplayStatics.GetPlayerCharacter` 0)))
      (bind _value (`/Game/Programming/Blueprints/Inventory/Spacial-System/SpacialInventoryComponent.QueryInventory` (`/Game/Programming/Blueprints/BP_MainCharacter.SpacialInventoryComponent` _asbp_main_character_2) (`KismetTextLibrary.Conv_StringToText` _objectiveid)))
      (`self.On Objective ID Heard` _objectiveid _value)))
  (`KismetSystemLibrary.Delay` 0.2)
  (bind _all_complete (`self.Are All Objectives Complete`))
  (set `self.IsCompleted` _all_complete))

(fn `Are All Objectives Complete`
  (returns (`All Complete` :type Boolean))
  (locals (`All Complete (local)` :type Boolean :default true))
  (bind (_currentstagedetails_stagename _currentstagedetails_description _currentstagedetails_objectives) (break `/Game/Programming/Blueprints/Questsystem/F_StageDetails` (`self.CurrentStageDetails`)))
  (for _array_element _currentstagedetails_objectives
    (bind (_objectivename _description _type _objectiveid) (break `/Game/Programming/Blueprints/Questsystem/F_ObjectiveDetails` _array_element))
    (if (not (>= (`BlueprintMapLibrary.Map_Find` (`self.CurrentObjectiveProgress`) _objectiveid) (`.Quantity_12_672DA79D4FCF4C63BD3CF6B9764C7F7D` (break `/Game/Programming/Blueprints/Questsystem/F_ObjectiveDetails` (`self.Get Objective Data By ID` _objectiveid)))))
      (bind _output_get (set `self.IsCompleted` false))
      (return _output_get)))
  (return (`local.All Complete (local)`)))

(fn `Get Objective Data By ID`
  (params (`Objective ID` :type String))
  (returns (`Objective Details` :type "/Game/Programming/Blueprints/Questsystem/F_ObjectiveDetails Structure"))
  (for _array_element (`.Objectives_20_0560FE6442A69F718DC381889D24ED81` (break `/Game/Programming/Blueprints/Questsystem/F_StageDetails` (`self.CurrentStageDetails`)))
    (if (`KismetStringLibrary.EqualEqual_StrStr` `Objective ID` (`.ObjectiveID_9_CBA8CABB4CD97AA856F7298588400C4D` (break `/Game/Programming/Blueprints/Questsystem/F_ObjectiveDetails` _array_element)))
      (return _array_element))))

(fn `Get Quest Details`
  (bind _returnvalue (`|GetDataTableRow` "/Game/Programming/Blueprints/Questsystem/QuestData.QuestData" (`self.QuestID`))
    (:`then`
      ;[1 1 1] fill quest details and stage details
      (bind _output_get (set `self.QuestDetails` _returnvalue))
      (bind _output_get_2 (set `self.CurrentStageDetails` (`|GetArrayItem` (`.Stages_14_FA8EA3FA40326E4DA55AAB864FF90D02` (break `/Game/Programming/Blueprints/Questsystem/F_QuestDetails` _output_get)) (`self.CurrentStage`))))
      ;[1 1 1] clear all objective progress
      (`BlueprintMapLibrary.Map_Clear` (`self.CurrentObjectiveProgress`))
      ;[1 1 1] add all the objectives with progress
      (for _array_element (`.Objectives_20_0560FE6442A69F718DC381889D24ED81` (break `/Game/Programming/Blueprints/Questsystem/F_StageDetails` _output_get_2))
        (`BlueprintMapLibrary.Map_Add` (`self.CurrentObjectiveProgress`) (`.ObjectiveID_9_CBA8CABB4CD97AA856F7298588400C4D` (break `/Game/Programming/Blueprints/Questsystem/F_ObjectiveDetails` _array_element)))))))

(fn `Is Objective Complete`
  (params (`Objective ID` :type String))
  (returns (ReturnValue :type Boolean))
  (bind _all_complete (`self.Are All Objectives Complete`))
  (set `self.IsCompleted` _all_complete)
  (return (>= (`BlueprintMapLibrary.Map_Find` (`self.CurrentObjectiveProgress`) (`local.Objective ID`)) (`.Quantity_12_672DA79D4FCF4C63BD3CF6B9764C7F7D` (break `/Game/Programming/Blueprints/Questsystem/F_ObjectiveDetails` (`self.Get Objective Data By ID` `Objective ID`))))))

(fn `On Objective ID Heard`
  (params (`Objective ID` :type String) (Value :type Integer :default 1))
  (bind (_value _returnvalue) (`BlueprintMapLibrary.Map_Find` (`self.CurrentObjectiveProgress`) (`local.Objective ID`)))
  (if (> (`KismetMathLibrary.SignOfInteger` Value) 0)
    (if _returnvalue
      (if true
        ;[1 1 1] increment current objective progress
        (`BlueprintMapLibrary.Map_Add` (`self.CurrentObjectiveProgress`) (`local.Objective ID`) (+ _value (`local.Value`)))
        (`self.Is Objective Complete` (`local.Objective ID`))
        (return))
      (else
        ;[1 1 1] this is not that quest
        (return)))
    (else
      ;[1 1 1] decreasing value
      (`BlueprintMapLibrary.Map_Add` (`self.CurrentObjectiveProgress`) (`local.Objective ID`) (+ (`BlueprintMapLibrary.Map_Find` (`self.CurrentObjectiveProgress`) (`local.Objective ID`)) (`local.Value`)))
      (return))))

(fn `UserConstructionScript`)