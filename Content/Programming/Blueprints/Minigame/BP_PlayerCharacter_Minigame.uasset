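; Player character for the hunting minigame, where the player aims and shoots at a foe loaded from the save game.
; Timelines drift the crosshair and animate aim size and speed while raising the foe's alert status.
; Shots land randomly inside the crosshair unless it is at minimum size, then line trace, max the next alert slot, apply damage and loot kills.
; A fleeing foe triggers a save and return to the forest level.
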(event `self.ReceiveBeginPlay`
  (bind _asbp_player_controller_minigame (cast `/Game/Programming/Blueprints/Minigame/BP_PlayerController_Minigame` (`GameplayStatics.GetPlayerController` 0)))
  (set `self.Controller_Ref` _asbp_player_controller_minigame)
  (bind _returnvalue (`GameplayStatics.DoesSaveGameExist` "save1"))
  (if _returnvalue
    ;[1 1 1] load game
    (bind (_inventorycontent _huntedfoe_alertstatus _huntedfoe_ref) (`/Game/Programming/Libraries_Enums_Interfaces/FL_Save.Load This Game` "save1" self (`self.InventoryComponent`)))
    (set `/Game/Programming/Blueprints/Inventory/InventoryComponent.Content` _inventorycontent (`self.InventoryComponent`))
    (set `self.FoeAlertStatus` _huntedfoe_alertstatus)
    (bind _returnvalue_2 (`GameplayStatics.GetActorOfClass` _huntedfoe_ref))
    (set `self.CurrentFightedFoe` _returnvalue_2)
    (set `self.CrosshairSize` (`self.MaxCrosshairSize`))
    (`self.StartPositionTimelime`)
    (else
      (`KismetSystemLibrary.PrintString` "Error: Save Game not Found" true true (struct :`R` 1.0 :`G` 0.020533 :`A` 1.0)))))

(event `StartPositionTimelime`
  (bind (_crosshairposition_x _crosshairposition_y) (`KismetMathLibrary.BreakVector2D` (`self.CrosshairPosition`)))
  ;[1 1 1] animate position
  (bind (_direction _position_offset) (`Timeline|Crosshair Position Timeline` :!via `PlayFromStart` :!label _label)
    (:`Update`
      (bind (_x _y) (`KismetMathLibrary.BreakVector3f` _position_offset))
      (set `self.CrosshairPosition` (`KismetMathLibrary.MakeVector2D` (+ _x _crosshairposition_x) (+ _y _crosshairposition_y))))
    (:`Finished`
      (if (`self.Debug_MovementShouldlLoop`)
        (`self.StartPositionTimelime`)))))

(event `StopPositionTimeline`
  (goto _label :!via `Stop`))

(event `StartAimAnimation`
  (bind _foealertstatus (`self.FoeAlertStatus`))
  ;[1 1 1] crosshair animation size
  (if (not (`self.FoeFledOrDied`))
    (bind (_direction _diameter _alertstatus _movement_speed) (`Timeline|Crosshair Aim Timeline` :`NewTime` (stale `Set New Aim Time To` NewTime) :!via `PlayFromStart` :!label _label_2)
      (:`Update`
        (set `self.CrosshairSize` _diameter)
        (set `self.CrosshairMovementSpeed` _movement_speed)
        ;[1 1 1 0.174] alert status
        ;;[1 1 1] find array index that is not 100 yet
        (for (_array_element _array_index) _foealertstatus
          (if (< _array_element 100.0)
            (break)))
        ;;[1 1 1] add numbers in that index
        (`KismetArrayLibrary.Array_Set` _foealertstatus _array_index (+ _array_element _alertstatus))
        (`/Game/Programming/Blueprints/FoeStuff/Foes/BP_FoeBase.UpdateAlertStatus` (`self.CurrentFightedFoe`) (`self.FoeAlertStatus`))))))

(event `StopAimAnimation`
  ;[1 1 1] crosshair animation size
  (goto _label_2 :!via `Stop`))

(event `Set New Aim Time To`
  (params (NewTime :type "Float (single-precision)"))
  ;[1 1 1] crosshair animation size
  (if (not (`self.FoeFledOrDied`))
    (goto _label_2 :!via `SetNewTime`)))

(event `self.ReceiveTick`
  (params (DeltaSeconds :type "Float (single-precision)"))
  (`/Game/Programming/Libraries_Enums_Interfaces/FL_Debug.PrintDebugMessage` "None" "Foe: " (`KismetSystemLibrary.GetDisplayName` (`self.CurrentFightedFoe`))))

(event `Foe Flees`
  (`/Game/Programming/Libraries_Enums_Interfaces/FL_Debug.PrintDebugMessage` "None" "Foe fled!" "" "" 10.0 "NewEnumerator13")
  (`self.Return To Forest`))

(fn `FillNextAlert`
  ;[1 1 1] check index 0
  (if (== (`|GetArrayItem` (`self.FoeAlertStatus`)) 100.0)
    ;[1 1 1] check index 1
    (if (== (`|GetArrayItem` (`self.FoeAlertStatus`) 1) 100.0)
      ;[1 1 1] check index 2
      (if (== (`|GetArrayItem` (`self.FoeAlertStatus`) 2) 100.0)
        (return)
        (else
          (`KismetArrayLibrary.Array_Set` (`self.FoeAlertStatus`) 2 100.0)))
      (else
        (`KismetArrayLibrary.Array_Set` (`self.FoeAlertStatus`) 1 100.0)))
    (else
      (`KismetArrayLibrary.Array_Set` (`self.FoeAlertStatus`) 0 100.0))))

(fn `FoeFledOrDied`
  (returns (ReturnValue :type Boolean))
  (bind _currentfightedfoe (`self.CurrentFightedFoe`))
  (return (or (`/Game/Programming/Blueprints/FoeStuff/Foes/BP_FoeBase.IsDead` _currentfightedfoe) (`/Game/Programming/Blueprints/FoeStuff/Foes/BP_FoeBase.IsFled` _currentfightedfoe))))

(fn `LineTraceBullet`
  (params (`Player Controller` :type "/Game/Programming/Blueprints/Minigame/BP_PlayerController_Minigame Object Reference") (`Shot Position` :type "Vector2D Structure"))
  (returns (OutHit :type "HitResult Structure") (ReturnValue :type Boolean))
  (locals (Offset_Local :type "Vector2D Structure"))
  (bind (_x _y) (`KismetMathLibrary.BreakVector2D` `Shot Position`))
  (bind (_returnvalue_x _returnvalue_y _returnvalue_z) (`KismetMathLibrary.BreakVector` (`SceneComponent.K2_GetComponentLocation` (`self.Camera`))))
  (`/Game/Programming/Libraries_Enums_Interfaces/FL_Debug.PrintDebugMessage` "None" "" "" "" 20.0 "NewEnumerator20")
  (bind (_outhit _returnvalue) (`KismetSystemLibrary.LineTraceSingle` :`Start` (`KismetMathLibrary.MakeVector` _returnvalue_x _returnvalue_y _returnvalue_z) :`End` (`KismetMathLibrary.MakeVector` 3000.0 (+ _returnvalue_y (* _x 7.4)) (+ _returnvalue_z (* _y -7.4))) :`TraceChannel` "TraceTypeQuery4" :`DrawDebugType` "Persistent" :`TraceColor` (struct :`R` 1.0 :`B` 0.761598 :`A` 1.0)))
  (return _outhit _returnvalue))

(fn `Move Crosshair Widget`
  (params (Position :type "Vector2D Structure"))
  (returns (`New Position` :type "Vector2D Structure"))
  (bind (_returnvalue_x _returnvalue_y) (`KismetMathLibrary.BreakVector2D` (* Position (`self.CrosshairMovementSpeed`))))
  (if (not (`self.FoeFledOrDied`))
    (switch `ECommonInputType` (`/Game/Programming/Blueprints/Minigame/BP_PlayerController_Minigame.CurrentInputType` (`self.Controller_Ref`))
      (:`MouseAndKeyboard`
        ;[1 1 1] dont invert
        (bind _output_get (set `self.CrosshairPosition` (+ (* Position (`self.CrosshairMovementSpeed`)) (`self.CrosshairPosition`))))
        (return _output_get))
      (:`Gamepad`
        ;[1 1 1] invert y axis
        (bind _output_get_2 (set `self.CrosshairPosition` (+ (`KismetMathLibrary.MakeVector2D` _returnvalue_x (* _returnvalue_y -1.0)) (`self.CrosshairPosition`))))
        (return _output_get_2)))))

(fn `PickUpItems`
  (params (Items :type "Array of /Game/Programming/Blueprints/Inventory/F_SlotStruct Structure"))
  (for _array_element Items
    (bind (_itemid _quantity) (break `/Game/Programming/Blueprints/Inventory/F_SlotStruct` _array_element))
    (`/Game/Programming/Blueprints/Inventory/InventoryComponent.AddToInventory` (`self.InventoryComponent`) _itemid _quantity)))

(fn `Return To Forest`
  (bind _success (`/Game/Programming/Libraries_Enums_Interfaces/FL_Save.Save This Game` "save1" (`self.InventoryComponent`) self (`self.FoeAlertStatus`) (`GameplayStatics.GetObjectClass` (`self.CurrentFightedFoe`))))
  (if _success
    (`GameplayStatics.OpenLevelBySoftObjectPtr` "/Game/Maps/Diorama_Lee.Diorama_Lee")))

(fn `ShootBullet`
  (params (Controller_Ref :type "/Game/Programming/Blueprints/Minigame/BP_PlayerController_Minigame Object Reference"))
  (returns (`Is Dead` :type Boolean) (`Shot Position` :type "Vector2D Structure"))
  (bind (_crosshairposition_x _crosshairposition_y) (`KismetMathLibrary.BreakVector2D` (`self.CrosshairPosition`)))
  (bind _returnvalue (`/Game/Programming/Blueprints/FoeStuff/Foes/BP_FoeBase.Check Is 0 HP` (`self.CurrentFightedFoe`)))
  ;[1 1 1] only shoot if foe isnt dead or has fled
  (if (not (`self.FoeFledOrDied`))
    ;[1 1 1] if crosshais is minimal size shot is accurate
    (if (== (`self.CrosshairSize`) (`self.MinCrosshairSize`))
      (set `self.ShotPosition` (`self.CrosshairPosition`))
      (else
        ;[1 1 1] if crosshair is not minimal size random point
        (bind (_x _y) (`/Game/Programming/Libraries_Enums_Interfaces/FL_Misc.Get Random Point In Circle` (`KismetMathLibrary.MakeVector` _crosshairposition_x _crosshairposition_y) 0.0 (/ (`self.CrosshairSize`) 2.0)))
        (bind _output_get (set `self.ShotPosition` (`KismetMathLibrary.MakeVector2D` _x _y)))))
    (bind _outhit (`self.LineTraceBullet` Controller_Ref _output_get))
    ;[1 1 1] update foe alert status
    (bind _alertstatus (`/Game/Programming/Blueprints/FoeStuff/Foes/BP_FoeBase.FillNextAlert` (`self.CurrentFightedFoe`)))
    (bind _output_get_2 (set `self.FoeAlertStatus` _alertstatus))
    (bind _fled (`/Game/Programming/Blueprints/FoeStuff/Foes/BP_FoeBase.UpdateAlertStatus` (`self.CurrentFightedFoe`) _output_get_2))
    (if (not _fled)
      ;[1 1 1] if foe has not fled and was hit apply damage
      (bind _asbp_foe_base (cast `/Game/Programming/Blueprints/FoeStuff/Foes/BP_FoeBase` (`.HitActor` (`GameplayStatics.BreakHitResult` _outhit)))
        (:`then`
          (bind _output_get_3 (set `self.CurrentFightedFoe` _asbp_foe_base))
          (`GameplayStatics.ApplyDamage` _output_get_3 (`self.Damage`) null self)
          ;[1 1 1] check if foe is dead and if it is pick up loot
          (if _returnvalue
            (`self.PickUpItems` (`/Game/Programming/Blueprints/FoeStuff/Foes/BP_FoeBase.Loot` (`self.CurrentFightedFoe`)))
            (return _returnvalue _output_get)
            (else
              (return false _output_get))))
        (:`CastFailed`
          (return false _output_get)))
      (else
        (`self.StopAimAnimation`)))))

(fn `UserConstructionScript`)