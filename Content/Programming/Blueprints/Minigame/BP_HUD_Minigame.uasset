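; BP_HUD_Minigame is the HUD for a shooting minigame, acting as a relay to its on-screen widget.
; On BeginPlay it caches the minigame controller and player character, then creates WB_MinigameHUDScreen with both references and adds it to the viewport.
; Its events forward crosshair size, crosshair position and shot positions to that widget.
; DisplayLoot only prints a debug message.
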(event `self.ReceiveBeginPlay`
  (bind _bp_controller (`self.BP_Controller`))
  ;[1 1 1] controller reference
  (bind _asbp_player_controller_minigame (cast `/Game/Programming/Blueprints/Minigame/BP_PlayerController_Minigame` (`self.GetOwningPlayerController`)))
  (set `self.BP_Controller` _asbp_player_controller_minigame)
  ;[1 1 1] player reference
  (bind _asbp_player_character_minigame (cast `/Game/Programming/Blueprints/Minigame/BP_PlayerCharacter_Minigame` (`GameplayStatics.GetPlayerCharacter` 0)))
  (set `self.BP_PlayerMinigame` _asbp_player_character_minigame)
  ;[1 1 1] create minigame hud
  (bind _returnvalue (`|CreateWidget` "/Game/Programming/Blueprints/Widgets/WB_MinigameHUDScreen.WB_MinigameHUDScreen_C" _bp_controller _bp_controller (`self.BP_PlayerMinigame`)))
  (bind _output_get (set `self.WB_MinigameHUD` _returnvalue))
  (`UserWidget.AddToViewport` _output_get 0))

(event `UpdateCrosshairSize`
  (params (Radius :type "Float (double-precision)"))
  (`/Game/Programming/Blueprints/Widgets/WB_MinigameHUDScreen.Update Size` (`self.WB_MinigameHUD`) Radius))

(event `UpdateCrosshairPosition`
  (params (InPosition :type "Vector2D Structure"))
  (`/Game/Programming/Blueprints/Widgets/WB_MinigameHUDScreen.Update Position` (`self.WB_MinigameHUD`) InPosition))

(event `Shoot Minigame`
  (params (InPosition :type "Vector2D Structure"))
  (`/Game/Programming/Blueprints/Widgets/WB_MinigameHUDScreen.ApplyBullet` (`self.WB_MinigameHUD`) InPosition))

(event `Display Loot`
  (`/Game/Programming/Libraries_Enums_Interfaces/FL_Debug.PrintDebugMessage` "None" "Display Loot" "" "" 10.0 "NewEnumerator14"))

(fn `UserConstructionScript`)