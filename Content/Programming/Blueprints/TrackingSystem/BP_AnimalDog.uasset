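; BP_AnimalDog is an AI-moved dog that follows the player character.
; On BeginPlay it casts player 0's character to BP_MainCharacter, caches it and starts FollowPlayer.
; FollowPlayer runs AIMoveTo toward the player with FollowDistance as the acceptance radius, re-calling itself only on success, so a failed move ends the loop.
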(event `self.ReceiveBeginPlay`
  (bind _asbp_main_character (cast `/Game/Programming/Blueprints/BP_MainCharacter` (`GameplayStatics.GetPlayerCharacter` 0)))
  (set `self.Player_Ref` _asbp_main_character)
  (`self.FollowPlayer`))

(event `FollowPlayer`
  ;[1 1 1] loop to follow player
  (bind _player_ref (`self.Player_Ref`)
    (:`then`
      (`|AIMoveTo` self (`self.K2_GetActorLocation` _player_ref) _player_ref (`self.FollowDistance`)
        (:`OnSuccess`
          (`self.FollowPlayer`))))
    (:`else`)))

(fn `UserConstructionScript`)