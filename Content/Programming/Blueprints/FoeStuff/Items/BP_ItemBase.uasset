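; BP_ItemBase is a base world pickup for items that go into the player's spatial inventory.
; On BeginPlay it fills a missing ItemObject from GetDefaultItemObject, which returns nothing at this level.
; Sphere overlaps show and collapse the WB_InteractPrompt widget through a direct cast, marked to become an interface.
; InteractWith tries to add the item to SpacialInventoryComponent, prints the result, and destroys the actor on success.
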(event `self.ReceiveBeginPlay`
  (`self.ItemObject`
    (:`then`)
    (:`else`
      (bind _itemobject (`self.GetDefaultItemObject`))
      (set `self.ItemObject` _itemobject))))

(event `self.Sphere.OnComponentBeginOverlap`
  (params (OverlappedComponent :type "PrimitiveComponent Object Reference") (OtherActor :type "Actor Object Reference") (OtherComp :type "PrimitiveComponent Object Reference") (OtherBodyIndex :type Integer) (bFromSweep :type Boolean) (SweepResult :type "HitResult Structure (by ref)"))
  ;[1 0 0] todo: make interface
  (bind _aswb_interact_prompt (cast `/Game/Programming/Blueprints/Widgets/WB_InteractPrompt` (`WidgetComponent.GetUserWidgetObject` (`self.InteractionPromtWidget`))))
  (`/Game/Programming/Blueprints/Widgets/WB_InteractPrompt.Set Visible` _aswb_interact_prompt))

(event `self.Sphere.OnComponentEndOverlap`
  (params (OverlappedComponent :type "PrimitiveComponent Object Reference") (OtherActor :type "Actor Object Reference") (OtherComp :type "PrimitiveComponent Object Reference") (OtherBodyIndex :type Integer))
  ;[1 0 0] todo: make interface
  (bind _aswb_interact_prompt (cast `/Game/Programming/Blueprints/Widgets/WB_InteractPrompt` (`WidgetComponent.GetUserWidgetObject` (`self.InteractionPromtWidget`))))
  (`/Game/Programming/Blueprints/Widgets/WB_InteractPrompt.Set Collapsed` _aswb_interact_prompt))

(event `InteractWith_1_1`
  (params (Player :type "/Game/Programming/Blueprints/BP_MainCharacter Object Reference")))

(fn `GetDefaultItemObject`
  (returns (ItemObject :type "/Game/Programming/Blueprints/Inventory/Spacial-System/BP_ItemObjectBase Object Reference"))
  (return null))

(fn `InteractWith`
  (params (Player :type "/Game/Programming/Blueprints/BP_MainCharacter Object Reference"))
  (returns (`Objective ID` :type String))
  (bind _itemobject (`self.ItemObject`))
  ;[1 1 1] try and add item to inventory
  (bind _added (`/Game/Programming/Blueprints/Inventory/Spacial-System/SpacialInventoryComponent.Try Add Item` (`/Game/Programming/Blueprints/BP_MainCharacter.SpacialInventoryComponent` Player) _itemobject))
  (`/Game/Programming/Libraries_Enums_Interfaces/FL_Debug.PrintDebugMessage` "None" "Added Item: " (`KismetStringLibrary.Conv_BoolToString` _added) "" 10.0 "NewEnumerator15")
  (if _added
    (`self.K2_DestroyActor`)
    (return (`KismetSystemLibrary.GetDisplayName` _itemobject))))

(fn `LookAt`
  (returns (Message :type Text))
  (return ""))

(fn `UserConstructionScript`)