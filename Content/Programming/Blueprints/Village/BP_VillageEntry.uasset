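; BP_VillageEntry is an interactable village entrance that prompts the player and lets them enter the village.
; InteractWith finds actors implementing I_HUDInterface, opens an interact prompt and returns an ID from inside that loop.
; Accept calls EnterVillage on the player, while Decline closes the prompt through the same interface lookup.
; LookAt returns empty text, and BeginPlay, overlap and Tick are unused.
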(event `InteractWith_1_1`
  (params (Player :type "/Game/Programming/Blueprints/BP_MainCharacter Object Reference")))

(event `/Game/Programming/Libraries_Enums_Interfaces/I_InteractInterface.Accept`
  (params (Player :type "/Game/Programming/Blueprints/BP_MainCharacter Object Reference"))
  (`/Game/Programming/Blueprints/BP_MainCharacter.Enter Village` Player))

(event `/Game/Programming/Libraries_Enums_Interfaces/I_InteractInterface.Decline`
  (params (Player :type "/Game/Programming/Blueprints/BP_MainCharacter Object Reference"))
  (bind _outactors (`GameplayStatics.GetAllActorsWithInterface` "/Game/Programming/Libraries_Enums_Interfaces/I_HUDInterface.I_HUDInterface_C"))
  (for _array_element _outactors
    (message `/Game/Programming/Libraries_Enums_Interfaces/I_HUDInterface.CloseInteractPrompt` _array_element)))

(fn `InteractWith`
  (params (Player :type "/Game/Programming/Blueprints/BP_MainCharacter Object Reference"))
  (returns (`Objective ID` :type String))
  (bind _outactors (`GameplayStatics.GetAllActorsWithInterface` "/Game/Programming/Libraries_Enums_Interfaces/I_HUDInterface.I_HUDInterface_C"))
  (for _array_element _outactors
    (message `/Game/Programming/Libraries_Enums_Interfaces/I_HUDInterface.OpenInteractPrompt` _array_element "NewEnumerator0")
    (return (`self.ID`))))

(fn `LookAt`
  (returns (Message :type Text))
  (return ""))

(fn `UserConstructionScript`)