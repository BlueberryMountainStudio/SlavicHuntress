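; Player controller that sets up overworld Enhanced Input and routes inventory and movement input.
; On BeginPlay it adds the overworld mapping context, then fetches BP_HUD through a macro that avoids an endless retry loop, printing an error on failure.
; Only after the HUD succeeds does it cache BP_MainCharacter via GetActorOfClass.
; The inventory action toggles the HUD inventory, and the move action forwards its value to the character.
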(event `self.ReceiveBeginPlay`
  (bind _returnvalue (subsystem `EnhancedInputLocalPlayerSubsystem`))
  ;[1 1 1] mapping contect
  (`/Engine/EditorBlueprintResources/StandardMacros.IsValid` _returnvalue
    (:`Is Valid`
      (`EnhancedInputSubsystemInterface.AddMappingContext` _returnvalue "/Game/Programming/InputMappings/InputMap_Overworld.InputMap_Overworld" 0 (struct))
      ;[1 1 1] using a macro so we dont have an infinite loop trying to access HUD class
      (bind _asbp_hud (`/Game/Programming/Libraries_Enums_Interfaces/BML_PlayerController.Get_BP_HUD` 10.0)
        (:`Success`
          (set `self.BP_HUD` _asbp_hud)
          ;[1 1 1] set up player character
          (bind _returnvalue_2 (`GameplayStatics.GetActorOfClass` "/Game/Programming/Blueprints/BP_MainCharacter.BP_MainCharacter_C"))
          (set `self.BP_MainCharacter_REF` _returnvalue_2))
        (:`Failed`
          (`/Game/Programming/Libraries_Enums_Interfaces/FL_Debug.PrintDebugMessage` "None" "Error: " "Unable to initialize BP_HUD" "" 1000.0 "NewEnumerator13"))))))

(event `EnhancedInput|/Game/Programming/InputMappings/IA_Inventory`
  (params (ActionValue :type Boolean) (ElapsedSeconds :type "Float (double-precision)") (TriggeredSeconds :type "Float (double-precision)") (InputAction :type "InputAction Object Reference" :default "/Game/Programming/InputMappings/IA_Inventory.IA_Inventory"))
  (:`Started`
    (`/Game/Programming/Blueprints/BP_HUD.Toggle Inventory` (`self.BP_HUD`))))

(event `EnhancedInput|/Game/Programming/InputMappings/IA_Move`
  (params (ActionValue :type "Vector2D Structure") (ElapsedSeconds :type "Float (double-precision)") (TriggeredSeconds :type "Float (double-precision)") (InputAction :type "InputAction Object Reference" :default "/Game/Programming/InputMappings/IA_Move.IA_Move"))
  (:`Triggered`
    (`/Game/Programming/Blueprints/BP_MainCharacter.Move` (`self.BP_MainCharacter_REF`) ActionValue)))

(fn `UserConstructionScript`)