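; BP_TrackBase is the base actor for an interactable track left by a foe, with an info widget showing that foe's track image.
; Cursor hover calls Hover, while main-character overlap with its sphere toggles an outline overlay and TrackInfoVisible.
; The first interaction freezes the player and switches the prompt to track info; a second calls StartTracking.
; Both starting and cancelling tracking restore movement and destroy the track, with no further tracking logic here.
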(event `self.ReceiveBeginPlay`)

(event `self.mesh.OnBeginCursorOver`
  (params (TouchedComponent :type "PrimitiveComponent Object Reference"))
  (if (not (`self.highlighted`))
    (`self.Hover` true)))

(event `self.mesh.OnEndCursorOver`
  (params (TouchedComponent :type "PrimitiveComponent Object Reference"))
  (`self.Hover` false))

(event `self.CollisionSphere.OnComponentBeginOverlap`
  (params (OverlappedComponent :type "PrimitiveComponent Object Reference") (OtherActor :type "Actor Object Reference") (OtherComp :type "PrimitiveComponent Object Reference") (OtherBodyIndex :type Integer) (bFromSweep :type Boolean) (SweepResult :type "HitResult Structure (by ref)"))
  (cast `/Game/Programming/Blueprints/BP_MainCharacter` OtherActor)
  (`MeshComponent.SetOverlayMaterial` (`self.mesh`) "/Game/Art/Props/Materials/Mat_Overlay_HighlightOutline.Mat_Overlay_HighlightOutline")
  (set `self.TrackInfoVisible` true))

(event `self.CollisionSphere.OnComponentEndOverlap`
  (params (OverlappedComponent :type "PrimitiveComponent Object Reference") (OtherActor :type "Actor Object Reference") (OtherComp :type "PrimitiveComponent Object Reference") (OtherBodyIndex :type Integer))
  (`MeshComponent.SetOverlayMaterial` (`self.mesh`) null)
  (set `self.TrackInfoVisible` false))

(event `/Game/Programming/Libraries_Enums_Interfaces/I_InteractInterface.InteractWith`
  (params (Player :type "/Game/Programming/Blueprints/BP_MainCharacter Object Reference"))
  ;[1 1 1] if interaction promt is displayed switch to info promt
  (if (== (`self.DisplayedInfoIndex`) 0)
    (set `/Game/Programming/Blueprints/BP_MainCharacter.CanMove` false Player)
    (set `self.TrackInfoVisible` true)
    (set `self.DisplayedInfoIndex` 1)
    (else
      ;[1 1 1] if info is already displayed start tracking the current track
      (`self.StartTracking` Player))))

(event `/Game/Programming/Libraries_Enums_Interfaces/I_InteractInterface.CancelInteraction`
  (params (Player :type "/Game/Programming/Blueprints/BP_MainCharacter Object Reference"))
  (`self.CancelTracking` Player))

(fn `CancelTracking`
  (params (Player :type "/Game/Programming/Blueprints/BP_MainCharacter Object Reference"))
  (set `/Game/Programming/Blueprints/BP_MainCharacter.CanMove` true Player)
  (`self.DestroySelf`)
  (return))

(fn `DestroySelf`
  (`self.K2_DestroyActor` self))

(fn `LookAt`
  (returns (Message :type Text))
  (return ""))

(fn `StartTracking`
  (params (Player :type "/Game/Programming/Blueprints/BP_MainCharacter Object Reference"))
  (set `/Game/Programming/Blueprints/BP_MainCharacter.CanMove` true Player)
  (`self.K2_DestroyActor` self))

(fn `Update Widget`
  (bind _aswb_track_info (cast `/Game/Programming/Blueprints/Widgets/WB_TrackInfo` (`WidgetComponent.GetUserWidgetObject` (`self.TrackInfo_Widget`))))
  (set `/Game/Programming/Blueprints/Widgets/WB_TrackInfo.Owner` self _aswb_track_info)
  (set `/Game/Programming/Blueprints/Widgets/WB_TrackInfo.Image` (`/Game/Programming/Blueprints/FoeStuff/Foes/BP_FoeBase.TrackImage` (`self.FoeSpawnedBy`)) _aswb_track_info))

(fn `UserConstructionScript`)