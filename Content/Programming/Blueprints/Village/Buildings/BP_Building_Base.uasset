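; Base village building actor that reacts to mouse hover and clicks on its mesh.
; On BeginPlay it caches all actors implementing I_VillageInterface.
; Cursor enter and exit toggle Hover, with exit also calling Highlight set to true.
; Hover and click events print debug messages with the mesh name, and clicking does nothing further.
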(event `self.ReceiveBeginPlay`
  (bind _outactors (`GameplayStatics.GetAllActorsWithInterface` "/Game/Programming/Libraries_Enums_Interfaces/I_VillageInterface.I_VillageInterface_C"))
  (set `self.AllActorsWithInterface` _outactors))

(event `self.mesh.OnBeginCursorOver`
  (params (TouchedComponent :type "PrimitiveComponent Object Reference"))
  ;[1 1 1] hover
  (`self.Hover` true)
  (`/Game/Programming/Libraries_Enums_Interfaces/FL_Debug.PrintDebugMessage` "House" "Hovered: " (`KismetSystemLibrary.GetDisplayName` (`self.mesh`)) "" 10.0))

(event `self.mesh.OnEndCursorOver`
  (params (TouchedComponent :type "PrimitiveComponent Object Reference"))
  ;[1 1 1] unhover
  (`self.Hover` false)
  (`self.Highlight` true))

(event `self.mesh.OnClicked`
  (params (TouchedComponent :type "PrimitiveComponent Object Reference") (ButtonPressed :type "Key Structure"))
  ;[1 1 1] click
  (`/Game/Programming/Libraries_Enums_Interfaces/FL_Debug.PrintDebugMessage` "House" "Clicked: " (`KismetSystemLibrary.GetDisplayName` (`self.mesh`)) "" 10.0))

(fn `UserConstructionScript`)