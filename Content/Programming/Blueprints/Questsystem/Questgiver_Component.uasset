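; Quest giver component that offers the quest referenced by its QuestData data table row when a player interacts with its owner.
; InteractWith checks the player's QuestlogComponent: an untracked quest has its name looked up and shown, while an active one reports that it is already taken.
; Display is debug messages only, with no quest acceptance here; InteractWith returns the owner's name and LookAt returns an empty string.
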(fn `Display Quest`
  (bind (_quest_data_datatable _quest_data_rowname) (break `DataTableRowHandle` (`self.Quest Data`)))
  (bind _returnvalue (`|GetDataTableRow` _quest_data_datatable _quest_data_rowname)
    (:`then`
      (`/Game/Programming/Libraries_Enums_Interfaces/FL_Debug.PrintDebugMessage` "None" (`KismetTextLibrary.Conv_TextToString` (`.QuestName_4_98D669254C893408A36861AD3062FF32` (break `/Game/Programming/Blueprints/Questsystem/F_QuestDetails` _returnvalue))) "" "" 10.0 "NewEnumerator15"))))

(fn `InteractWith`
  (params (Player :type "/Game/Programming/Blueprints/BP_MainCharacter Object Reference"))
  (returns (`Objective ID` :type String))
  (bind (_quest_data_datatable _quest_data_rowname) (break `DataTableRowHandle` (`self.Quest Data`)))
  (bind _returnvalue (`KismetSystemLibrary.GetDisplayName` (`self.GetOwner`)))
  (if (not (`/Game/Programming/Blueprints/Questsystem/Questlog_Component.Query Active Quest` (`/Game/Programming/Blueprints/BP_MainCharacter.Questlog_Component` (`/Game/Programming/Libraries_Enums_Interfaces/FL_Misc.GetMyPlayerCharacter`)) _quest_data_rowname))
    (`self.Display Quest`)
    (return _returnvalue)
    (else
      (`/Game/Programming/Libraries_Enums_Interfaces/FL_Debug.PrintDebugMessage` "Quest" "Already on Quest: " (`KismetStringLibrary.Conv_NameToString` _quest_data_rowname) "" 20.0 "NewEnumerator20")
      (return _returnvalue))))

(fn `LookAt`
  (returns (Message :type Text))
  (return ""))