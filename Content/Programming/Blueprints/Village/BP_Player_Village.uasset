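; BP_Player_Village is the village player Blueprint that moves the game from the village to the hunt.
; The EnterHunt event and a debug-style 5 key shortcut both open the Diorama_Lee level directly.
; Save and load logic for the "save1" slot, covering inventory and settings, is present but disconnected, so the transition does not save and BeginPlay does nothing.
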(event `self.ReceiveBeginPlay`)

(event `Key|Five`
  (params (Key :type "Key Structure"))
  (:`Pressed`
    (`GameplayStatics.OpenLevelBySoftObjectPtr` "/Game/Maps/Diorama_Lee.Diorama_Lee" :!label _label)))

(event `Enter Hunt`
  (goto _label))

(fn `UserConstructionScript`)