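; Inventory component that lets its owner look at and interact with items; adding to and removing from the inventory are empty stubs.
; Every tick a debug-drawn sphere trace along the owner's forward vector caches the hit actor, calling its LookAt interface message and printing the result when the target changes.
; The interact input passes that actor to a server event, which sends an interact message to its ItemDataComponent, if present.
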(event `self.ReceiveTick`
  (params (DeltaSeconds :type "Float (single-precision)"))
  (`self.InteractionTrace`))

(event `EnhancedInput|/Game/Programming/InputMappings/IA_Interact`
  (params (ActionValue :type Boolean) (ElapsedSeconds :type "Float (double-precision)") (TriggeredSeconds :type "Float (double-precision)") (InputAction :type "InputAction Object Reference" :default "/Game/Programming/InputMappings/IA_Interact.IA_Interact"))
  (:`Started`
    (bind _lookatactor (`self.LookAtActor`)
      (:`then`
        (`self.Server_Interact` _lookatactor))
      (:`else`))))

(event `Server_Interact`
  (params (Target :type "Actor Object Reference"))
  (bind _returnvalue (`Actor.GetComponentByClass` Target "/Game/Programming/Blueprints/Inventory/ItemDataComponent.ItemDataComponent_C"))
  ;[0 0.8645 1] the tutorial made it server side but idk if its necessary
  ;[1 1 1] check if the actor we look at has a ItemDataComponent
  (`/Engine/EditorBlueprintResources/StandardMacros.IsValid` _returnvalue
    (:`Is Valid`
      (message `/Game/Programming/Libraries_Enums_Interfaces/I_InteractInterface.InteractWith` _returnvalue))))

(fn `AddToInventory`)

(fn `InteractionTrace`
  (bind _returnvalue (`self.GetOwner`))
  (bind _returnvalue_2 (`Actor.K2_GetActorLocation` _returnvalue))
  (bind (_outhit _returnvalue_3) (`KismetSystemLibrary.SphereTraceSingle` _returnvalue_2 (+ _returnvalue_2 (* (`Actor.GetActorForwardVector` _returnvalue) (`self.InteractionRange`))) 15.0 "TraceTypeQuery3" false (`|MakeArray` (`self.GetOwner`)) "ForOneFrame"))
  (if _returnvalue_3
    (bind (_bblockinghit _binitialoverlap _time _distance _location _impactpoint _normal _impactnormal _physmat _hitactor) (`GameplayStatics.BreakHitResult` _outhit))
    ;[1 1 1] check if looked at actor changed
    (if (!= (`self.LookAtActor`) _hitactor)
      ;[1 1 1] try to call LookAt for the actor the owner looks at, if said actor doesnt implement the interaction interface nothing happens
      (bind _output_get (set `self.LookAtActor` _hitactor))
      (bind _message (message `/Game/Programming/Libraries_Enums_Interfaces/I_InteractInterface.LookAt` _output_get))
      (`/Game/Programming/Libraries_Enums_Interfaces/FL_Debug.PrintDebugMessage` "None" "Looking At: " (`KismetTextLibrary.Conv_TextToString` _message) "" 10.0 "NewEnumerator18"))
    (else
      (set `self.LookAtActor` null))))

(fn `RemoveFromInventory`)